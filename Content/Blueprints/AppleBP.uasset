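; Apple item Blueprint for a Snake game, with a Speedup behaviour component and a timed self-destruction.
; Both are configured from values on the Snake game mode through overridable configure events.
; The game mode's change-tick percentage becomes a fraction on the Speedup component, and its apple lifetime sets the item's self-destruction time.
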(event ConfigureBehaviourComponent(Speedup)
  (bind _returnvalue (Class|ItemBase|GetSnakeGameMode))
  (Variables|/Script/MrsSnake.SpeedupComponent|SetChangeTickPercent (Variables|Default|GetSpeedup) (/ (Math|Conversions|ToFloat(Integer) (Class|MrsSnakeGameModeBase|GetChangeTickPercent _returnvalue)) 1e+02)))

(event EventConfigureItem
  (bind _returnvalue (Class|ItemBase|GetSnakeGameMode))
  (Variables|Default|SetSelfDestructionTime self (Math|Conversions|ToFloat(Integer) (Class|MrsSnakeGameModeBase|GetAppleLifeTime _returnvalue))))

(fn ConstructionScript)